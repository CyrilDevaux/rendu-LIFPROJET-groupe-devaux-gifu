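; BP_Personnage is a team-based combat character that attacks other characters, takes damage and dies.
; TeamIsSet tints team 1 blue and binds the attack, damage and death dispatchers.
; Attacking another BP_Personnage fires its damage dispatcher and reports an AI damage event; each hit removes fixed health, notifying GameInstanceV1 at zero, while the death dispatcher destroys the actor.
; Older movement and AI state-reset logic remains unconnected, alongside debug prints.
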(event `TeamIsSet`
  (if (== (`self.Equipe`) 1)
    ;[1 1 1] Pour differencier les deux équipes
    (`PrimitiveComponent.SetMaterial` (`self.Mesh`) 0 "/Game/LevelPrototyping/Materials/MI_Solid_Blue.MI_Solid_Blue"))
  (add `self.Dead` (delegate `destroy self`))
  (add `self.DamageReceive` (delegate `decreaseHealth`))
  ;[1 1 1] Quand on reçoit l'information Attacked (un peu comme un appel de fonction)
  (add `self.Attack` (delegate `CustomEvent`)))

(event `decreaseHealth` :!signature `self.DamageReceive`
  (params (`damage dealer` :type "Actor Object Reference"))
  (bind _output_get (set `self.CurrentHealth` (- (`self.CurrentHealth`) 10)))
  (`KismetSystemLibrary.PrintString` (`KismetStringLibrary.Conv_IntToString` _output_get))
  (`KismetSystemLibrary.PrintString` "from")
  (`KismetSystemLibrary.PrintString` (`KismetSystemLibrary.GetDisplayName` `damage dealer`))
  (if (<= _output_get 0)
    (`KismetSystemLibrary.PrintString` "debut mort" true true (struct :`R` 1.0 :`G` 0.523797 :`B` 0.073567 :`A` 1.0) 5.0)
    (bind _asgame_instance_v1 (cast `/Game/GameInstanceV1` (`GameplayStatics.GetGameInstance`))
      (:`then`
        (`/Game/GameInstanceV1.EnnemyDeath` _asgame_instance_v1 self))
      (:`CastFailed`
        (`KismetSystemLibrary.PrintString` "CAST TO GAME INSTANCE FAILED (in bp_personnage event dispatcher attack" true true (struct :`R` 1.0 :`A` 1.0) 10.0)))))

(event `destroy self`
  (`KismetSystemLibrary.PrintString` "fin mort" true true (struct :`R` 1.0 :`G` 0.283589 :`B` 0.109966 :`A` 1.0) 5.0)
  (`self.K2_DestroyActor`))

(event `CustomEvent` :!signature `self.Attack`
  (params (Enemy :type "Actor Object Reference"))
  (bind _returnvalue (`GameplayStatics.GetObjectClass` Enemy))
  (if (`KismetMathLibrary.ClassIsChildOf` _returnvalue "BP_Personnage_C")
    (if (`KismetSystemLibrary.IsValid` Enemy)
      (bind _asbp_personnage (cast `/Game/BP_Personnage` Enemy)
        (:`then`
          (`self.DamageReceive` _asbp_personnage self)
          (`AISense_Damage.ReportDamageEvent` Enemy self))
        (:`CastFailed`
          (`KismetSystemLibrary.PrintString` "CAST TO BP_PERSONNAGE FAILED (in bp_personnage event dispatcher Attack)" true true (struct :`R` 1.0 :`A` 1.0) 10.0))))
    (else
      (`KismetSystemLibrary.PrintString` "PAS BP_PERSONNAGE !!" true true (struct :`R` 1.0 :`B` 0.143874 :`A` 1.0) 23.0)
      (if (`KismetMathLibrary.ClassIsChildOf` _returnvalue "/Game/AI_Personnage.AI_Personnage_C")
        (`KismetSystemLibrary.PrintString` "AI_personnage" true true (struct :`R` 1.0 :`B` 0.037156 :`A` 1.0) 232.0)
        (else
          (`KismetSystemLibrary.PrintString` (`KismetSystemLibrary.GetDisplayName` Enemy)))))))

(fn `give moveTo location`
  (returns (NextLocation :type "Vector Structure") (CurrentLocation :type "Vector Structure"))
  (bind _returnvalue (`self.K2_GetActorLocation`))
  (bind _result (`/Engine/EditorBlueprintResources/StandardMacros.NegateFloat` (.y _returnvalue))
    (:`  `
      (return (`KismetMathLibrary.MakeVector` (.x _returnvalue) _result (.z _returnvalue)) _returnvalue))))

(fn `UserConstructionScript`)